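; Throwable drone tool that waters and temporarily freezes nearby Burnt_Base actors, then restores some of their health.
; After a short delay on spawn it reveals its cone and cylinder and scales up the effect with a timeline.
; When scaling finishes, one capsule trace around the drone finds targets to freeze and water.
; Seconds later it unfreezes and heals that same cached hit list, then destroys itself.
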(event `self.ReceiveBeginPlay`
  (bind _returnvalue (`SceneComponent.K2_GetComponentLocation` (`self.DroneMesh`)))
  (`KismetSystemLibrary.Delay` 1.3)
  (`SceneComponent.SetVisibility` (`self.Cone`) true false)
  (`SceneComponent.SetVisibility` (`self.Cylinder`) true false)
  (bind (_direction _scale) (`Timeline|ScaleTimeline`)
    (:`Update`
      (`SceneComponent.SetRelativeScale3D` (`self.Scene`) (* (`self.ScaleSize`) _scale)))
    (:`Finished`
      (bind _outhits (`KismetSystemLibrary.CapsuleTraceMultiForObjects` :`Start` (+ _returnvalue (0.0 0.0 10.0)) :`End` (+ _returnvalue (0.0 0.0 -10.0)) :`Radius` 500.0 :`HalfHeight` 400.0 :`ObjectTypes` (`|MakeArray` "ObjectTypeQuery2" "ObjectTypeQuery1" :!type "EObjectTypeQuery Enum") :`DrawTime` 3.0))
      (for _array_element _outhits
        (bind _asburnt_base (cast `/Game/Blueprints/GameObjects/Burnables/Burnt_Base` (`.HitActor` (`GameplayStatics.BreakHitResult` _array_element))))
        (set `/Game/Blueprints/GameObjects/Burnables/Burnt_Base.isFrozen` true _asburnt_base)
        (`/Game/Blueprints/GameObjects/Burnables/Burnt_Base.Water` _asburnt_base 1500.0))
      (`KismetSystemLibrary.Delay` 9.0)
      (for _array_element_2 _outhits
        (bind _asburnt_base_2 (cast `/Game/Blueprints/GameObjects/Burnables/Burnt_Base` (`.HitActor` (`GameplayStatics.BreakHitResult` _array_element_2))))
        (set `/Game/Blueprints/GameObjects/Burnables/Burnt_Base.isFrozen` false _asburnt_base_2)
        (set `/Game/Blueprints/GameObjects/Burnables/Burnt_Base.HealthCurrent` (`KismetMathLibrary.FClamp` (+ (`/Game/Blueprints/GameObjects/Burnables/Burnt_Base.HealthCurrent` _asburnt_base_2) 2000.0) 0.0 (`/Game/Blueprints/GameObjects/Burnables/Burnt_Base.HealthMax` _asburnt_base_2)) _asburnt_base_2))
      (`self.K2_DestroyActor`))))

(fn `UserConstructionScript`)