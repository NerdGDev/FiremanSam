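; SWFF game mode that runs a match, optionally timed, and opens EndLevel when it finishes.
; BeginPlay resets the game instance and waits briefly before enabling tick and recording the start time.
; If the Timer flag is set, a looping one-second event updates the countdown and ends the match when time expires or the game instance's TotalBurning reaches zero.
; Tick writes both players' pawn locations into the PlayerLocations material parameter collection.
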(event `self.ReceiveBeginPlay`
  (`WidgetBlueprintLibrary.SetInputMode_GameOnly` (`GameplayStatics.GetPlayerController` 0))
  (bind _asswffgame_instance (cast `/Game/Blueprints/GameModes/SWFFGameInstance` (`GameplayStatics.GetGameInstance`)))
  (`/Game/Blueprints/GameModes/SWFFGameInstance.Reset` _asswffgame_instance)
  (`self.SetActorTickEnabled` false)
  (`KismetSystemLibrary.Delay` 4.0)
  (`self.SetActorTickEnabled` true)
  (`self.StartGame`))

(event `self.ReceiveTick`
  (params (DeltaSeconds :type "Float (single-precision)"))
  (bind _returnvalue (`GameplayStatics.GetPlayerPawn` 1))
  (bind _returnvalue_2 (`GameplayStatics.GetPlayerPawn` 0))
  (`|ExecutionSequence`
    (:`then_0`
      (if (`KismetSystemLibrary.IsValid` _returnvalue_2)
        (`KismetMaterialLibrary.SetVectorParameterValue` "/Game/Materials/CommonUseMPC/PlayerLocations.PlayerLocations" "Player1" (make `LinearColor` (.x (`self.K2_GetActorLocation` _returnvalue_2)) (.y (`self.K2_GetActorLocation` _returnvalue_2)) (.z (`self.K2_GetActorLocation` _returnvalue_2))))))
    (:`then_1`
      (if (`KismetSystemLibrary.IsValid` _returnvalue)
        (`KismetMaterialLibrary.SetVectorParameterValue` "/Game/Materials/CommonUseMPC/PlayerLocations.PlayerLocations" "Player2" (make `LinearColor` (.x (`self.K2_GetActorLocation` _returnvalue)) (.y (`self.K2_GetActorLocation` _returnvalue)) (.z (`self.K2_GetActorLocation` _returnvalue))))))))

(event `StartGame`
  (set `self.TimeStart` (`GameplayStatics.GetTimeSeconds`))
  (if (`self.Timer`)
    (`KismetSystemLibrary.K2_SetTimerDelegate` (delegate `Time`) 1.0 true)))

(event `Time`
  (bind _output_get (set `self.GameTimespan` (`KismetMathLibrary.MakeTimespan` 0 0 0 (`KismetMathLibrary.FTrunc` (- (`self.TimeTotal`) (- (`GameplayStatics.GetTimeSeconds`) (`self.TimeStart`)))))))
  (bind _asswffgame_instance (cast `/Game/Blueprints/GameModes/SWFFGameInstance` (`GameplayStatics.GetGameInstance`)))
  (if (or (== (`/Game/Blueprints/GameModes/SWFFGameInstance.TotalBurning` _asswffgame_instance) 0) (and (<= (`KismetMathLibrary.GetSeconds` _output_get) 0) (<= (`KismetMathLibrary.GetMinutes` _output_get) 0)))
    (`GameplayStatics.OpenLevel` "EndLevel")))

(fn `UserConstructionScript`)